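; BP_SceneReflectMirror is a mirror actor that fakes a reflection with a scene capture by following the player camera's view direction.
; Every tick it negates the camera forward vector's X and Y, converts it to a rotation, then adds a fixed pitch offset and flipped roll.
; SceneCaptureCamera and SceneCapturePane both receive that world rotation; only orientation updates, ignoring player position.
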(event `self.ReceiveTick`
  (params (DeltaSeconds :type "Float (single-precision)"))
  (bind _returnvalue (`KismetMathLibrary.MakeRot` (+ (.pitch (`KismetMathLibrary.Conv_VectorToRotator` (* (`KismetMathLibrary.GetForwardVector` (`PlayerCameraManager.GetCameraRotation` (`PlayerController.PlayerCameraManager` (`GameplayStatics.GetPlayerController` 0)))) (-1.0 -1.0 1.0)))) 10.0) (.yaw (`KismetMathLibrary.Conv_VectorToRotator` (* (`KismetMathLibrary.GetForwardVector` (`PlayerCameraManager.GetCameraRotation` (`PlayerController.PlayerCameraManager` (`GameplayStatics.GetPlayerController` 0)))) (-1.0 -1.0 1.0)))) 180.0))
  (`SceneComponent.K2_SetWorldRotation` (`self.SceneCaptureCamera`) _returnvalue false)
  (`SceneComponent.K2_SetWorldRotation` (`self.SceneCapturePane`) _returnvalue false))

(fn `UserConstructionScript`)