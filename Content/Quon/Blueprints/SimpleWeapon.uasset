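; SimpleWeapon is a basic gun Blueprint that fires Bullet projectiles, with its ammo logic left as stubs.
; Shoot spawns a Bullet at the supplied actor location plus GunOffset rotated by control rotation, then plays a fire sound there.
; It returns AmmoInGun without decrementing or checking it.
; GetCurrentAmmo, GetMaxAmmo and Reload only return zero, and the event graph and construction script are empty.
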(event `self.ReceiveBeginPlay`)

(event `self.ReceiveActorBeginOverlap`
  (params (OtherActor :type "Actor Object Reference")))

(event `self.ReceiveTick`
  (params (DeltaSeconds :type "Float (single-precision)")))

(fn `GetCurrentAmmo`
  (returns (CurrentAmmo :type Integer))
  (return 0))

(fn `GetMaxAmmo`
  (returns (MaxAmmo :type Integer))
  (return 0))

(fn `Reload`
  (returns (CurrentAmmo :type Integer))
  (return 0))

(fn `Shoot`
  (params (PawnControlRotation :type "Object.Rotator Structure") (ActorLocation :type "Object.Vector Structure"))
  (returns (Ammunition :type Integer))
  (bind _returnvalue (+ ActorLocation (`KismetMathLibrary.GreaterGreater_VectorRotator` (`self.GunOffset`) PawnControlRotation)))
  (`|SpawnActorFromClass` "/Game/Quon/Props/Bullet.Bullet_C" (`KismetMathLibrary.MakeTransform` _returnvalue PawnControlRotation)) ; Spawn projectile
  (`GameplayStatics.PlaySoundAtLocation` "/Game/FirstPersonBP/Audio/FirstPerson_WeaponFire.FirstPerson_WeaponFire" _returnvalue) ; Play firing sound
  (return (`self.AmmoInGun`)))

(fn `UserConstructionScript`)